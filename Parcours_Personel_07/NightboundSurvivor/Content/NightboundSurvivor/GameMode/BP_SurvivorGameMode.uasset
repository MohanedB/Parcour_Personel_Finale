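; Game mode for Nightbound Survivor that sets up the HUD and runs the pause-for-upgrade flow.
; BeginPlay adds the HUD widget to the first player's viewport.
; OnUpgradeAvailable opens and stores an upgrade menu, pauses the game and shows the cursor; CloseUpgradeMenu removes that menu, unpauses and hides it.
; Input mode switch nodes are present but never wired in, so input mode stays unchanged.
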(event `self.ReceiveBeginPlay`
  (bind _returnvalue (`|CreateWidget` "/Game/NightboundSurvivor/UI/WBP_HUD.WBP_HUD_C" (`GameplayStatics.GetPlayerController` 0)))
  (`UserWidget.AddToViewport` _returnvalue 0))

(event `self.OnUpgradeAvailable`
  (bind _returnvalue (`|CreateWidget` "/Game/NightboundSurvivor/UI/WBP_UpgradeMenu.WBP_UpgradeMenu_C" (`GameplayStatics.GetPlayerController` 0)))
  (bind _output_get (set `self.CurrentUpgradeMenu` _returnvalue))
  (`UserWidget.AddToViewport` _output_get 0)
  (`GameplayStatics.SetGamePaused` true)
  (set `PlayerController.bShowMouseCursor` true (`GameplayStatics.GetPlayerController` 0)))

(event `CloseUpgradeMenu`
  (`Widget.RemoveFromParent` (`self.CurrentUpgradeMenu`))
  (`GameplayStatics.SetGamePaused` false)
  (set `PlayerController.bShowMouseCursor` false (`GameplayStatics.GetPlayerController` 0)))

(fn `UserConstructionScript`)