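; GA_RaycastAttack is a Gameplay Ability that performs a hitscan attack for Nightbound Survivor.
; On activation it line-traces on the Visibility channel a fixed distance along the avatar's forward vector, with debug drawing left on.
; On a hit, it applies a SurvivorDamageEffect spec from the owner's ability system component to the hit actor's.
; The graph never calls CommitAbility or EndAbility.
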(event `self.K2_ActivateAbility`
  (bind _returnvalue (`self.GetAvatarActorFromActorInfo`))
  (bind _returnvalue_2 (`self.GetAbilitySystemComponentFromActorInfo`))
  (bind _returnvalue_3 (`Actor.K2_GetActorLocation` _returnvalue))
  (bind (_outhit _returnvalue_4) (`KismetSystemLibrary.LineTraceSingle` :`Start` _returnvalue_3 :`End` (+ _returnvalue_3 (* (`Actor.GetActorForwardVector` _returnvalue) 1000.0)) :`TraceChannel` "TraceTypeQuery1" :`DrawDebugType` "ForDuration"))
  (if _returnvalue_4
    (`AbilitySystemComponent.BP_ApplyGameplayEffectSpecToTarget` _returnvalue_2 (`AbilitySystemComponent.MakeOutgoingSpec` :`self` _returnvalue_2 :`GameplayEffectClass` "/Script/NightboundSurvivor.SurvivorDamageEffect") (`AbilitySystemBlueprintLibrary.GetAbilitySystemComponent` (`.HitActor` (`GameplayStatics.BreakHitResult` _outhit))))))